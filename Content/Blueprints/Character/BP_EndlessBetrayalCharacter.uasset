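; Player character Blueprint for Endless Betrayal, whose live logic shows and hides the sniper scope overlay.
; ShowSniperScopeWidget lazily creates and caches WBP_SniperScope, then plays its zoom animation forward or reversed with a matching 2D zoom sound.
; BeginPlay, Tick and the construction script are empty.
; Leftover debug logic for server-side back-and-forth movement and an overhead net-role display is disconnected and never runs.
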(event EventBeginPlay)

(event Collision|EventActorBeginOverlap
  (params (OtherActor :type Actor%20Object%20Reference)))

(event EventTick
  (params (DeltaSeconds :type Float%20%28single-precision%29))
  ;[1 1 1] Makes the Server player move back and forth for DEbug purpose
)

(event EventShowSniperScopeWidget
  (params (bShouldShowScope :type Boolean))
  (Variables|Default|GetSniper%20Scope%20Widget%20Ref
    (:then
      _)
    (:else
      (bind _returnvalue (UserInterface|CreateWidget "/Game/Blueprints/HUD/WBP_SniperScope.WBP_SniperScope_C"))
      (bind _output_get (Variables|Default|SetSniper%20Scope%20Widget%20Ref _returnvalue))
      (UserInterface|Viewport|AddtoViewport _output_get 0)))
  (if bShouldShowScope
    (bind _sniper_scope_widget_ref (Variables|Default|GetSniper%20Scope%20Widget%20Ref)
      (:then
        (UserInterface|Animation|PlayAnimation _sniper_scope_widget_ref (Variables|/Game/Blueprints/HUD/WBP_SniperScope.WBP_SniperScope_C|GetScopeZoomIn _sniper_scope_widget_ref) 0.0 1 "Forward" 1.0 false)
        (Audio|PlaySound2D "/Game/Assets/MilitaryWeapSilver/Sound/SniperRifle/Cues/SniperRifle_ZoomIn_Cue.SniperRifle_ZoomIn_Cue" 1.0 1.0 0.0 0 0))
      (:else))
    (else
      (bind _sniper_scope_widget_ref_2 (Variables|Default|GetSniper%20Scope%20Widget%20Ref)
        (:then
          (UserInterface|Animation|PlayAnimation _sniper_scope_widget_ref_2 (Variables|/Game/Blueprints/HUD/WBP_SniperScope.WBP_SniperScope_C|GetScopeZoomIn _sniper_scope_widget_ref_2) 0.0 1 "Reverse" 1.0 false)
          (Audio|PlaySound2D "/Game/Assets/MilitaryWeapSilver/Sound/SniperRifle/Wavs/SniperRifle_ZoomOut.SniperRifle_ZoomOut" 1.0 1.0 0.0 0 0))
        (:else)))))

(fn ConstructionScript)